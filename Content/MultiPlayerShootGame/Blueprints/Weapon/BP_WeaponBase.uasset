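; BP_WeaponBase is the base weapon pickup actor for a multiplayer shooter, starting as a physics object with ammo initialized from weapon info.
; On authority, its collision sphere selects an overlapping player who didn't just drop it and offers the weapon unless their inventory holds that type.
; It retries every 0.2 seconds until interactable, and ending overlap updates the player's DroppedWeapon.
; On player death, it detaches, re-enables physics and pickup queries, and is thrown forward.
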(event OnComponentBeginOverlap(CollisionSphere)
  (params (OverlappedComponent :type Primitive%20Component%20Object%20Reference) (OtherActor :type Actor%20Object%20Reference) (OtherComp :type Primitive%20Component%20Object%20Reference) (OtherBodyIndex :type Integer) (bFromSweep :type Boolean) (SweepResult :type Hit%20Result%20Structure%20%28by%20ref%29))
  (bind _overlappingactors (Collision|GetOverlappingActors "/Game/MultiPlayerShootGame/Blueprints/Player/BP_PlayerBase.BP_PlayerBase_C" :!class /Script/Engine.Actor))
  (if (Actor|ActorHasTag OtherActor "Player")
    (Networking|SwitchHasAuthority
      (:Authority
        (if (Variables|Default|GetbCanBeInteractedWith) :!label _label
          (if (> (Utilities|Array|Length _overlappingactors) 1)
            (bind _array_element (Utilities|Array|ForEachLoopwithBreak _overlappingactors :!label _label_2)
              (:LoopBody
                (bind _playerbaseref (Class|INTPlayerBase|GetPlayerBaseRef(Message) _array_element))
                (if (!= (Variables|/Game/MultiPlayerShootGame/Blueprints/Player/BP_PlayerBase.BP_PlayerBase_C|GetDroppedWeapon _playerbaseref) self)
                  (Variables|Default|SetInteractingPlayer _playerbaseref)
                  (goto _label_2 Break)))
              (:Completed
                (bind _array_element_2 (Utilities|Array|ForEachLoopwithBreak (Variables|/Game/MultiPlayerShootGame/Blueprints/Player/BP_PlayerBase.BP_PlayerBase_C|GetWeaponInventory (stale _interactingplayer)) :!label _label_3)
                  (:LoopBody
                    (if (Utilities|Enum|Equal(Enum) (.Type (Utilities|Struct|BreakST_WeaponInfo (CallFunction|FGetWeaponInfo (Variables|BP_WeaponBase_C|GetWeaponName _array_element_2)))) (.Type (Utilities|Struct|BreakST_WeaponInfo (CallFunction|FGetWeaponInfo (Variables|Default|GetWeaponName)))))
                      (Variables|/Game/MultiPlayerShootGame/Blueprints/Player/BP_PlayerBase.BP_PlayerBase_C|SetbCouldLootWeapon (Variables|Default|GetInteractingPlayer) false)
                      (goto _label_3 Break)))
                  (:Completed
                    (if (Variables|/Game/MultiPlayerShootGame/Blueprints/Player/BP_PlayerBase.BP_PlayerBase_C|GetbCouldLootWeapon (stale _interactingplayer))
                      (Default|AddOverlapWeapon (Variables|Default|GetInteractingPlayer) self)
                      (else
                        (Variables|/Game/MultiPlayerShootGame/Blueprints/Player/BP_PlayerBase.BP_PlayerBase_C|SetbCouldLootWeapon (Variables|Default|GetInteractingPlayer) true)))))))
            (elif (== (Utilities|Array|Length _overlappingactors) 1)
              (bind _playerbaseref_2 (Class|INTPlayerBase|GetPlayerBaseRef(Message) (Utilities|Array|Get(acopy) _overlappingactors)))
              (Utilities|IsValid _playerbaseref_2
                (:Is%20Valid
                  (if (!= (Variables|/Game/MultiPlayerShootGame/Blueprints/Player/BP_PlayerBase.BP_PlayerBase_C|GetDroppedWeapon _playerbaseref_2) self)
                    (Variables|Default|SetInteractingPlayer _playerbaseref_2)
                    (bind _interactingplayer (Variables|Default|GetInteractingPlayer)
                      (:then
                        (goto _label_3))
                      (:else)))))))
          (else
            (Utilities|FlowControl|Delay 0.2)
            (goto _label)))))))

(event OnComponentEndOverlap(CollisionSphere)
  (params (OverlappedComponent :type Primitive%20Component%20Object%20Reference) (OtherActor :type Actor%20Object%20Reference) (OtherComp :type Primitive%20Component%20Object%20Reference) (OtherBodyIndex :type Integer))
  (if (Actor|ActorHasTag OtherActor "Player")
    (Networking|SwitchHasAuthority
      (:Authority
        (bind _playerbaseref (Class|INTPlayerBase|GetPlayerBaseRef(Message) OtherActor))
        (Default|SetDroppedWeapon _playerbaseref)))))

(event Custom|SVR_InitWeaponAmmo
  (bind _weaponname (Variables|Default|GetWeaponName))
  (bind _weaponinfo (CallFunction|FGetWeaponInfo _weaponname))
  (bind (_maxammoinmag _maxextraammo) (Utilities|Struct|BreakST_WeaponInfo _weaponinfo))
  (Variables|Default|SetCurrentMagAmmo _maxammoinmag)
  (Variables|Default|SetCurrentExtraAmmo _maxextraammo))

(event Custom|SVR_DropWeaponWhenPlayerDead
  (params (PlayerForwardVector :type Vector%203f%20Structure))
  (bind (_x _y _z) (Class|KismetMathLibrary|BreakVector3f PlayerForwardVector))
  (bind _weapon (Variables|Default|GetWeapon))
  (Transformation|DetachFromActor "KeepWorld" "KeepWorld" "KeepWorld")
  (Collision|SetCollisionEnabled _weapon "PhysicsOnly")
  (Physics|SetSimulatePhysics _weapon true)
  (Collision|SetCollisionEnabled (Variables|Default|GetCollisionSphere) "QueryOnly")
  (Physics|AddImpulse (Variables|Default|GetWeapon) (Math|Vector|MakeVector (* _x 6e+02) (* _y 6e+02) _z) "None" true))

(event EventBeginPlay
  (Physics|SetSimulatePhysics (Variables|Default|GetWeapon) true)
  (CallFunction|SVRInitWeaponAmmo))

(fn ConstructionScript)

(fn GetWeaponBaseRef
  (return self))