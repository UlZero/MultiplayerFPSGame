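; Game mode for a round-based Terrorist versus Counter-Terrorist multiplayer shooter that handles spawning, team scores and chat.
; Players spawn at random team spawn points gathered on login and are tracked in alive and dead maps by team class.
; Each death triggers a team headcount; a wiped team scores the round, announces the winner to spawned players and respawns them after a delay.
; Chat messages enter a capped history that is pushed to spawned players' controllers.
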(event Custom|RequestSpawnPlayerCharacter
  (params (PlayerController :type BPPC%20Player%20Controler%20Object%20Reference) (Class :type Actor%20Class%20Reference))
  (Default|SpawnPlayerCharacter PlayerController Class (Math|Transform|SelectTransform (Transformation|GetActorTransform (.OutItem (Utilities|Array|Random (Variables|Default|GetTerroristSP)))) (Transformation|GetActorTransform (.OutItem (Utilities|Array|Random (Variables|Default|GetCounterTerroristSP)))) (== Class "/Game/MultiPlayerShootGame/Blueprints/Player/BP_PlayerTerrorist.BP_PlayerTerrorist_C"))))

(event Custom|AddDeadPlayer
  (params (Player :type BP%20Player%20Base%20Object%20Reference%20%28by%20ref%29))
  (if (.ReturnValue (Utilities|Map|Find (Variables|Default|GetPlayerAlive) Player))
    (Utilities|Map|Remove (Variables|Default|GetPlayerAlive) Player))
  (bind _playercontrollerref (Class|INTPlayerController|GetPlayercontrollerRef(Message) (Pawn|GetController Player)))
  (Utilities|Map|Add (Variables|Default|GetPlayerDead) Player (Variables|/Game/MultiPlayerShootGame/Blueprints/BPPC_PlayerControler.BPPC_PlayerControler_C|GetTeamClass _playercontrollerref))
  (bind (_conterterroristalive _terroristalive) (Utilities|MCheckNumOfLivePlayer)
    (:Completed
      (if (or (== _conterterroristalive 0) (== _terroristalive 0))
        (CallFunction|FCalculateTeamScore)
        (for _array_element (Variables|Default|GetPlayerSpawned)
          (bind _playercontrollerref_2 (Class|INTPlayerController|GetPlayercontrollerRef(Message) (Pawn|GetController _array_element)))
          (bind _values (Utilities|Map|Values (Variables|Default|GetPlayerAlive)))
          (Default|WinAnucment _playercontrollerref_2 (Utilities|Array|Get(acopy) _values) (Variables|Default|GetDisplay%20Time) (select (== (Utilities|Array|Get(acopy) _values) "/Game/MultiPlayerShootGame/Blueprints/Player/BP_PlayerCounterTerrorist.BP_PlayerCounterTerrorist_C") (Variables|Default|GetCTScore) (Variables|Default|GetTeScore))))
        (Utilities|Map|Clear (Variables|Default|GetPlayerDead))
        (Utilities|Map|Clear (Variables|Default|GetPlayerAlive))
        (Utilities|FlowControl|Delay (Variables|Default|GetDisplay%20Time))
        (for _array_element_2 (Variables|Default|GetPlayerSpawned)
          (Default|SVRAddtoAlivePlayer _array_element_2)
          (Default|ReSpawn _array_element_2))))))

(event Custom|AddAlivePlayer
  (params (Player :type BP%20Player%20Base%20Object%20Reference%20%28by%20ref%29))
  (if (.ReturnValue (Utilities|Map|Find (Variables|Default|GetPlayerDead) Player))
    (Utilities|Map|Remove (Variables|Default|GetPlayerDead) Player))
  (bind _playercontrollerref (Class|INTPlayerController|GetPlayercontrollerRef(Message) (Pawn|GetController Player)))
  (Utilities|Map|Add (Variables|Default|GetPlayerAlive) Player (Variables|/Game/MultiPlayerShootGame/Blueprints/BPPC_PlayerControler.BPPC_PlayerControler_C|GetTeamClass _playercontrollerref)))

(event Custom|UpdateGameMeassage
  (params (Meassage :type Text%20%28by%20ref%29))
  ;[1 1 1] GameMeassageRoutine
  (if (Utilities|Text|TextIsEmpty Meassage)
    _
    (else
      (bind _returnvalue (Utilities|Array|Add (Variables|Default|GetGameMeassage) Meassage))
      (if (> _returnvalue (Variables|Default|GetGameMeassageCount)) :!label _label
        (Utilities|Array|RemoveIndex (Variables|Default|GetGameMeassage))
        (goto _label)
        (else
          _))))
  (for _array_element (Variables|Default|GetPlayerSpawned)
    (bind _playercontrollerref (Class|INTPlayerController|GetPlayercontrollerRef(Message) (Pawn|GetController _array_element)))
    (Utilities|IsValid _playercontrollerref
      (:Is%20Valid
        (Default|UpdateChatBox _playercontrollerref (Variables|Default|GetGameMeassage))))))

(event Custom|AddSpawnedPlayer
  (params (NewItem :type BP%20Player%20Base%20Object%20Reference%20%28by%20ref%29))
  (Utilities|Array|Add (Variables|Default|GetPlayerSpawned) NewItem))

(event EventOnLogout
  (params (ExitingController :type Controller%20Object%20Reference))
  (bind _playerbaseref (Class|INTPlayerBase|GetPlayerBaseRef(Message) (Pawn|GetControlledPawn ExitingController)))
  (Utilities|IsValid _playerbaseref
    (:Is%20Valid
      (Utilities|Array|RemoveItem (Variables|Default|GetPlayerSpawned) _playerbaseref))))

(event EventPostLogin
  (params (NewPlayer :type Player%20Controller%20Object%20Reference))
  (Utilities|Array|AddUnique (Variables|Default|GetPlayerController) NewPlayer)
  (bind _outactors (Actor|GetAllActorsOfClass "/Game/MultiPlayerShootGame/Blueprints/SpawnPoints/BP_TerroristSP.BP_TerroristSP_C"))
  (Variables|Default|SetTerroristSP _outactors)
  (bind _outactors_2 (Actor|GetAllActorsOfClass "/Game/MultiPlayerShootGame/Blueprints/SpawnPoints/BP_CounterTerroristSP.BP_CounterTerroristSP_C"))
  (Variables|Default|SetCounterTerroristSP _outactors_2))

(fn ConstructionScript)

(fn FCalculateTeamScore
  (if (== (Variables|Default|GetConterTerroristAlive) 0)
    (Math|Integer|IncrementInt (Variables|Default|GetTeScore))
    (else
      (Math|Integer|IncrementInt (Variables|Default|GetCTScore)))))

(fn FGetGameModeRef
  (return self))